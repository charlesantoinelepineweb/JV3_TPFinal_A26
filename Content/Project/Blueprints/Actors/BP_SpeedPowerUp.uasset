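; BP_SpeedPowerUp is a pickup actor that triggers a speed effect on the collecting player's opponents rather than on the collector.
; When a BP_PlatformingCharacter overlaps its sphere, it reads that character's PlayerNumber and loops over all platforming characters.
; Any character with a different number receives ApplySpeedEffect, and the pickup destroys itself, so it stays if no such character exists.
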(event OnComponentBeginOverlap(Sphere1)
  (params (OverlappedComponent :type Primitive%20Component%20Object%20Reference) (OtherActor :type Actor%20Object%20Reference) (OtherComp :type Primitive%20Component%20Object%20Reference) (OtherBodyIndex :type Integer) (bFromSweep :type Boolean) (SweepResult :type Hit%20Result%20Structure%20%28by%20ref%29))
  (Development|PrintString "Overlap  vitesse detecte")
  (bind _asbp_platforming_character (Utilities|Casting|CastToBP_PlatformingCharacter OtherActor))
  (Variables|Default|SetCollectPlayerNumber (Variables|/Game/Variant_Platforming/Blueprints/BP_PlatformingCharacter.BP_PlatformingCharacter_C|GetPlayerNumber _asbp_platforming_character))
  (bind _outactors (Actor|GetAllActorsOfClass "/Game/Variant_Platforming/Blueprints/BP_PlatformingCharacter.BP_PlatformingCharacter_C"))
  (for _array_element _outactors
    (bind _asbp_platforming_character_2 (Utilities|Casting|CastToBP_PlatformingCharacter _array_element))
    (if (!= (Variables|/Game/Variant_Platforming/Blueprints/BP_PlatformingCharacter.BP_PlatformingCharacter_C|GetPlayerNumber _asbp_platforming_character_2) (Variables|Default|GetCollectPlayerNumber))
      (Development|PrintString "Joueur 2 detecter")
      (Default|ApplySpeedEffect _asbp_platforming_character_2)
      (Actor|DestroyActor))))

(fn ConstructionScript)