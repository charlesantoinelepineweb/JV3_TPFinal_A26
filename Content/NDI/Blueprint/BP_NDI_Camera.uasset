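; BP_NDI_Camera is a camera Blueprint that outputs a scene capture over NDI.
; On BeginPlay it points SceneCaptureNDI at a render target, creates a media capture from NDIOutput and starts capturing that render target.
; An on-screen message in French reports success or failure.
; On EndPlay it stops the media capture if it is still valid.
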(event EventBeginPlay
  (Variables|/Script/Engine.SceneCaptureComponent2D|SetTextureTarget (Variables|Default|GetSceneCapture_NDI) (Variables|Default|GetRenderTarget))
  (bind _returnvalue (Class|MediaOutput|CreateMediaCapture (Variables|Default|GetNDI_Output)))
  (bind _output_get (Variables|Default|SetMediaCaptureActive _returnvalue))
  (bind _returnvalue_2 (Class|MediaCapture|CaptureTextureRenderTarget2D _output_get (Variables|Default|GetRenderTarget)))
  (if _returnvalue_2
    (Development|PrintString "Capture NDI Démarré" true true "(R=0.000000,G=0.660000,B=1.000000,A=1.000000)" 5.0)
    (else
      (Development|PrintString "ÉCHEC" true true "(R=1.000000,G=0.000000,B=0.034279,A=1.000000)" 5.0))))

(event EventEndPlay
  (params (EndPlayReason :type EEndPlayReason%20Enum :default "Destroyed"))
  (bind _mediacaptureactive (Variables|Default|GetMediaCaptureActive))
  (Utilities|IsValid _mediacaptureactive
    (:Is%20Valid
      (Class|MediaCapture|StopCapture _mediacaptureactive false))))

(fn ConstructionScript)